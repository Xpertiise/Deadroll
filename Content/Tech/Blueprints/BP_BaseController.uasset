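; BP_BaseController is a base player controller that sets up the game's master UI.
; On BeginPlay it creates WBP_UIMaster, adds it to the viewport, shows the mouse cursor and switches input to UI only.
; It then hands the widget to the game mode through PassUIMessage.
; Getter functions expose the UI widget and, through DiceBoxRef, a stored variable still named NewVar.
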(event EventBeginPlay
  (bind _returnvalue (UserInterface|CreateWidget "/Game/UI/WBP_UIMaster.WBP_UIMaster_C" self))
  (bind _output_get (Variables|Default|SetUI _returnvalue))
  (UserInterface|Viewport|AddtoViewport _output_get 0)
  (Variables|Default|SetbShowMouseCursor true)
  (Input|SetInputModeUIOnly self 0 "DoNotLock" false)
  (Class|BPIGamemode|PassUI(Message) (Game|GetGameMode) (Variables|Default|GetUI)))

(fn ConstructionScript)

(fn DiceBoxRef
  (return (Variables|Default|GetNewVar)))

(fn GetUI
  (return (Variables|Default|GetUI)))