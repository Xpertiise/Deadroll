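; BP_DiceSpawner is an actor that spawns the physical dice for a given set of die data.
; SpawnDice destroys the previous dice, then spawns a Standard, Weighted, Explosive or Mirrored die Blueprint per entry, chosen by DieType.
; Each die appears half-scale at a jittered position with random rotation, receiving the spawner, static mesh origin and its index.
; Init stores a GameManager reference.
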(event Custom|SpawnDice
  (params (Count :type Array%20of%20S%20Dice%20Structures))
  (Variables|Default|SetDiceRef Count)
  (for _array_element (Variables|Default|GetDiceObj)
    (Actor|DestroyActor _array_element))
  (Utilities|Array|Clear (Variables|Default|GetDiceObj))
  (for _index (range 1 (Utilities|Array|Length (Variables|Default|GetDiceRef)))
    (bind _returnvalue (Game|SpawnActorfromClass (Utilities|Select :Index (Utilities|Struct|BreakS_Dice (Utilities|Array|Get(acopy) (Variables|Default|GetDiceRef) (- _index 1))) :NewEnumerator0 "/Game/Tech/Blueprints/BP_StandardDice.BP_StandardDice_C" :NewEnumerator1 "/Game/Tech/Blueprints/BP_WeightedDice.BP_WeightedDice_C" :NewEnumerator2 "/Game/Tech/Blueprints/BP_ExplosiveDice.BP_ExplosiveDice_C" :NewEnumerator3 "/Game/Tech/Blueprints/BP_MirrorDice.BP_MirrorDice_C") (Math|Transform|MakeTransform (+ (Transformation|GetActorLocation self) (Math|Vector|MakeVector (Math|Random|RandomFloatinRange -17.0 17.0) (Math|Random|RandomFloatinRange -17.0 17.0) (Math|Random|RandomFloatinRange -17.0 17.0))) (Math|Random|RandomRotator true) "0.500000,0.500000,0.500000") "AdjustIfPossibleButAlwaysSpawn" "MultiplyWithRoot" 0 self (Transformation|GetWorldLocation (Variables|Default|GetStaticMesh)) (- _index 1) 0))
    (Utilities|Array|Add (Variables|Default|GetDiceObj) _returnvalue)))

(event Custom|Init
  (params (GameManager :type BP%20Game%20Manager%20Object%20Reference))
  (Variables|Default|SetGameManager GameManager))

(fn ConstructionScript)