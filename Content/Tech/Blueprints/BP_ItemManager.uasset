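; Item manager that runs the shop and player inventory in a dice game.
; Init sorts DT_Items rows into rarity pools, and GenerateShop fills slots by weighted rarity rolls, re-rolling duplicates through the NewRarity event.
; The item-obtained dispatcher triggers purchases, which check and deduct GameManager currency, add to inventory, refresh dice and notify UI through dispatchers.
; One item phase routes through OnPickup, where Sir Cal Bluff becomes a random owned item.
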(event Custom|Init
  (EventDispatchers|BindEventtoEDItemObtained (delegate Custom|CustomEvent))
  (bind _outrownames (DataTable|GetDataTableRowNames "/Game/Tech/Data/DT_Items.DT_Items"))
  (for _array_element _outrownames
    (bind _returnvalue (Utilities|GetDataTableRow "/Game/Tech/Data/DT_Items.DT_Items" _array_element)
      (:then
        (switch Utilities|FlowControl|Switch|SwitchonE_ItemRarity (.rarity _returnvalue)
          (:NewEnumerator0
            (Utilities|Array|Add (Variables|Default|GetCommonItems) (Utilities|Struct|MakeS_ItemData (.rarity _returnvalue) (.itemtype _returnvalue) (.id _returnvalue) (.itemname _returnvalue) (.itemdescription _returnvalue) (.cost _returnvalue) (.effectvalue _returnvalue) (.itemphase _returnvalue) (.onetime _returnvalue))))
          (:NewEnumerator1
            (Utilities|Array|Add (Variables|Default|GetUncommonItems) (Utilities|Struct|MakeS_ItemData (.rarity _returnvalue) (.itemtype _returnvalue) (.id _returnvalue) (.itemname _returnvalue) (.itemdescription _returnvalue) (.cost _returnvalue) (.effectvalue _returnvalue) (.itemphase _returnvalue) (.onetime _returnvalue))))
          (:NewEnumerator2
            (Utilities|Array|Add (Variables|Default|GetRareItems) (Utilities|Struct|MakeS_ItemData (.rarity _returnvalue) (.itemtype _returnvalue) (.id _returnvalue) (.itemname _returnvalue) (.itemdescription _returnvalue) (.cost _returnvalue) (.effectvalue _returnvalue) (.itemphase _returnvalue) (.onetime _returnvalue)))))))))

(event Custom|GenerateShop
  (for _index (range 1 (Variables|Default|GetShopItemCount))
    (CallFunction|AddItemstoShop))
  (Default|CallEDShopGenerated (Variables|Default|GetCurrentShopItems)))

(event Custom|ClearShop
  (Utilities|Array|Clear (Variables|Default|GetCurrentShopItems))
  (Default|CallEDShopClear))

(event Custom|NewRarity
  (CallFunction|AddItemstoShop))

(event Custom|CustomEvent
  (params (Item :type S%20Item%20Data%20Structure) (ItemIndex :type Integer))
  (CallFunction|BuyItemFunct Item ItemIndex))

(fn ConstructionScript)

(fn GenerateRarity
  (bind _returnvalue (Math|Random|RandomFloatinRange 0.0 1.0))
  (if (<= _returnvalue 0.1)
    (LocalVariables|SetTargetRarity "NewEnumerator2")
    (elif (<= _returnvalue 0.4)
      (LocalVariables|SetTargetRarity "NewEnumerator1")
      (else
        (LocalVariables|SetTargetRarity "NewEnumerator0"))))
  (return (LocalVariables|GetTargetRarity)))

(fn AddItemstoShop
  (bind _uncommonitems (Variables|Default|GetUncommonItems))
  (bind _rareitems (Variables|Default|GetRareItems))
  (bind _commonitems (Variables|Default|GetCommonItems))
  (bind _outitem (Utilities|Array|Random _rareitems))
  (bind _outitem_2 (Utilities|Array|Random _commonitems))
  (bind _outitem_3 (Utilities|Array|Random _uncommonitems))
  (bind _rarity (CallFunction|GenerateRarity))
  (switch Utilities|FlowControl|Switch|SwitchonE_ItemRarity _rarity
    (:NewEnumerator0
      (if (Utilities|Array|ContainsItem (Variables|Default|GetCurrentShopItems) _outitem_2)
        (CallFunction|NewRarity)
        (else
          (Utilities|Array|Add (Variables|Default|GetCurrentShopItems) _outitem_2))))
    (:NewEnumerator1
      (if (Utilities|Array|ContainsItem (Variables|Default|GetCurrentShopItems) _outitem_3)
        (CallFunction|NewRarity)
        (else
          (Utilities|Array|Add (Variables|Default|GetCurrentShopItems) _outitem_3))))
    (:NewEnumerator2
      (if (Utilities|Array|ContainsItem (Variables|Default|GetCurrentShopItems) _outitem)
        (CallFunction|NewRarity)
        (else
          (Utilities|Array|Add (Variables|Default|GetCurrentShopItems) _outitem))))))

(fn GetRandomUpgrades)

(fn OnPickup
  (params (CheckedItem :type S%20Item%20Data%20Structure))
  (bind (_id _itemphase) (Utilities|Struct|BreakS_ItemData CheckedItem))
  (bind _inventory (Variables|Default|GetInventory))
  (bind _returnvalue (Utilities|Array|LastIndex _inventory))
  (bind _returnvalue_2 (Math|Random|RandomIntegerinRange 0 _returnvalue))
  (bind _output (Utilities|Array|Get(acopy) _inventory _returnvalue_2))
  (if (Utilities|Enum|Equal(Enum) _itemphase "NewEnumerator8")
    (switch Utilities|FlowControl|Switch|SwitchonE_ItemID _id
      (:NewEnumerator18
        (bind _output_get (LocalVariables|SetOutputItemRef _output))
        (Development|PrintString (Utilities|String|Append "Duplicated: " (.ItemName (Utilities|Struct|BreakS_ItemData _output))))
        (return _output_get)))
    (else
      (return CheckedItem))))

(fn BuyItemFunct
  (params (InputPin :type S%20Item%20Data%20Structure) (InputPin2 :type Integer))
  (bind _cost (Utilities|Struct|BreakS_ItemData InputPin))
  (bind _gamemanager (Variables|Default|GetGameManager))
  (bind _gamedata (Variables|/Game/Tech/Blueprints/BP_GameManager.BP_GameManager_C|GetGameData _gamemanager))
  (bind _currentcurrency (Utilities|Struct|BreakS_UIStruct _gamedata))
  (if (>= _currentcurrency _cost)
    (LocalVariables|SetNewLocalVar true)
    (Default|CallEDonCurrencyChanged (Variables|Default|GetGameManager) (* _cost -1))
    (Utilities|Struct|SetmembersinS_UIStruct _gamedata (- _currentcurrency _cost))
    (Utilities|Array|SetArrayElem :TargetArray (Variables|Default|GetCurrentShopItems) :Index InputPin2)
    (if (Utilities|Enum|Equal(Enum) (Utilities|Struct|BreakS_ItemData InputPin) "NewEnumerator8")
      (bind _outputitem (CallFunction|OnPickup InputPin))
      (Utilities|Array|Add (Variables|Default|GetInventory) _outputitem)
      (else
        (Utilities|Array|Add (Variables|Default|GetInventory) InputPin)))
    (Default|CallEDShopUpdated InputPin2)
    (Default|DiceSetup (Variables|Default|GetGameManager))
    (Default|CallEDInventoryUpdated (Variables|Default|GetGameManager) InputPin)
    (Audio|PlaySound2D (.OutItem (Utilities|Array|Random (Variables|Default|GetSFX))) 1.0 1.0 0.0 0 0)
    (return (LocalVariables|GetNewLocalVar))
    (else
      (LocalVariables|SetNewLocalVar false)
      (Development|PrintString "Broke boy"))))

(fn ClearInventory
  (bind _gamemanager (Variables|Default|GetGameManager))
  (bind _ui (Variables|/Game/Tech/Blueprints/BP_GameManager.BP_GameManager_C|GetUI _gamemanager))
  (bind _wbp_inventory (Variables|/Game/UI/WBP_UIMaster.WBP_UIMaster_C|GetWBP_Inventory _ui))
  (bind _inventoryitems (Variables|/Game/UI/WBP_Inventory.WBP_Inventory_C|GetInventoryItems _wbp_inventory))
  (Utilities|Array|Clear (Variables|Default|GetInventory))
  (for _array_element _inventoryitems
    (Widget|RemovefromParent _array_element))
  (Utilities|Array|Clear _inventoryitems))