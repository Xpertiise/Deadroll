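; Explosive die Blueprint, a child die whose effect fires the settled event on the DiceManager through DiceEffect.
; Construction gives its point light a dynamic pulsing light-function material with a random offset, so instances pulse out of sync.
; An unconnected chain holds a delayed burst on a roll of six, with Niagara effect, radial impulse and torque, but it never runs.
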(event EventBeginPlay
  (|CallParentFunction))

(event EventDiceEffect
  (Default|CallEDDieSettled (Variables|Default|GetDiceManager)))

(fn ConstructionScript
  (|CallParentFunction)
  (bind _returnvalue (Rendering|Material|CreateDynamicMaterialInstance "/Game/Art/LightMaterials/M_PulsingLight.M_PulsingLight" "None" "None" :!class /Script/Engine.KismetMaterialLibrary))
  (Rendering|Components|Light|SetLightFunctionMaterial (Variables|Default|GetPointLight) _returnvalue)
  (Rendering|Material|SetScalarParameterValue _returnvalue "Offset" (Math|Random|RandomFloatinRange 0.0 0.5) :!class /Script/Engine.MaterialInstanceDynamic))