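; Dice manager that spawns the physical dice for a roll and detects when all of them have settled.
; SpawnDice replaces existing dice with standard, weighted, explosive or mirrored actors, randomly rotated and scattered around a plane.
; Settle events are counted until all dice report, then a full-settle event fires.
; That event updates the highest non-mirrored roll before running each die's after-settle effect.
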(event Custom|SpawnDice
  (params (DiceRef :type Array%20of%20S%20Dice%20Structures))
  (Variables|Default|SetDiceRef DiceRef)
  (for _array_element (Variables|Default|GetDiceObj)
    (Actor|DestroyActor _array_element))
  (Utilities|Array|Clear (Variables|Default|GetDiceObj))
  (for _index (range 1 (Utilities|Array|Length (Variables|Default|GetDiceRef)))
    (bind _returnvalue (Game|SpawnActorfromClass (Utilities|Select :Index (Utilities|Struct|BreakS_Dice (Utilities|Array|Get(acopy) (Variables|Default|GetDiceRef) (- _index 1))) :NewEnumerator0 "/Game/Tech/Blueprints/Dice/BP_StandardDice.BP_StandardDice_C" :NewEnumerator1 "/Game/Tech/Blueprints/Dice/BP_WeightedDice.BP_WeightedDice_C" :NewEnumerator2 "/Game/Tech/Blueprints/Dice/BP_ExplosiveDice.BP_ExplosiveDice_C" :NewEnumerator3 "/Game/Tech/Blueprints/Dice/BP_MirrorDice.BP_MirrorDice_C") (Math|Transform|MakeTransform (+ (Transformation|GetWorldLocation (Variables|Default|GetPlane)) (Math|Vector|MakeVector (Math|Random|RandomFloatinRange -1e+01 1e+01) (Math|Random|RandomFloatinRange -1e+01 1e+01) (Math|Random|RandomFloatinRange -1e+01 3e+01))) (Math|Random|RandomRotator true) "1.300000,1.300000,1.300000") "AdjustIfPossibleButAlwaysSpawn" "MultiplyWithRoot" 0 self (- _index 1) (Transformation|GetWorldLocation (Variables|Default|GetStaticMesh)) 0))
    (Utilities|Array|Add (Variables|Default|GetDiceObj) _returnvalue)))

(event Custom|Init
  (params (GameManager :type BP%20Game%20Manager%20Object%20Reference))
  (Variables|Default|SetGameManager GameManager)
  (EventDispatchers|BindEventtoEDDieSettled (delegate Custom|DieSettled))
  (EventDispatchers|BindEventtoEDFullSettle (delegate Custom|FullSettle)))

(event Custom|DieSettled
  (CallFunction|Settled))

(event Custom|FullSettle
  (params (DiceRef :type Array%20of%20BP%20Standard%20Dice%20Object%20References))
  (Variables|Default|SetSettledDice 0)
  (for _array_element (Variables|Default|GetDiceObj)
    (Utilities|GetHighestRoll _array_element))
  (for _array_element_2 DiceRef
    (Default|AfterSettleEffect _array_element_2)))

(event Custom|Clear
  (for _array_element (Variables|Default|GetDiceObj)
    (Actor|DestroyActor _array_element))
  (Utilities|Array|Clear (Variables|Default|GetDiceObj)))

(fn ConstructionScript)

(fn Settled
  (bind _result (Math|Integer|IncrementInt (Variables|Default|GetSettledDice))
    (:%20%20
      (if (== _result (Utilities|Array|Length (Variables|Default|GetDiceRef)))
        (Default|CallEDFullSettle (Variables|Default|GetDiceObj))
        (Variables|Default|SetSettledDice 0)))))