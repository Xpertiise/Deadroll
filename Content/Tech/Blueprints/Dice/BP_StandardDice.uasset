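; BP_StandardDice is a physics-rolled die with no special effect, launched on BeginPlay with a randomized impulse and torque.
; A looping timer waits for near-zero velocity, then maps the highest mesh socket to a face value.
; The result is written into the GameManager's HeldDice entry before DiceEffect notifies DiceManager of settling.
; A UI event pops the die upward, shows its score widget and increments score; overlaps play random dice sounds.
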(event OnComponentBeginOverlap(Box)
  (params (OverlappedComponent :type Primitive%20Component%20Object%20Reference) (OtherActor :type Actor%20Object%20Reference) (OtherComp :type Primitive%20Component%20Object%20Reference) (OtherBodyIndex :type Integer) (bFromSweep :type Boolean) (SweepResult :type Hit%20Result%20Structure%20%28by%20ref%29))
  (if (Utilities|Enum|Equal(Enum) (Collision|GetCollisionObjectType OtherComp) "ECC_WorldDynamic")
    (Audio|PlaySound2D (.OutItem (Utilities|Array|Random (Utilities|Array|MakeArray "/Game/Audio/Dice1.Dice1" "/Game/Audio/Dice2.Dice2" "/Game/Audio/Dice3.Dice3" "/Game/Audio/Dice4.Dice4" "/Game/Audio/Dice5.Dice5"))) 1.0 1.0 0.0 0 0)))

(event Custom|SetStatic
  (Utilities|IsVelocityLowEnough
    (:True
      (Variables|Default|SetStatic true)
      (bind _finalvalue (CallFunction|SetRolls))
      (Utilities|SetRefs _finalvalue)
      (CallFunction|DiceEffect)
      (Utilities|Time|ClearandInvalidateTimerbyHandle (Variables|Default|GetTimer)))))

(event Custom|UI
  (bind _value (Variables|Default|GetValue))
  (Development|PrintString (Utilities|String|ToString(Integer) (Variables|Default|GetValue)))
  (Physics|AddForce (Variables|Default|GetCube) "0.000000,0.000000,25000.000000" "None" true)
  (Class|PrimitiveComponent|SetPhysMaterialOverride (Variables|Default|GetCube) "/Game/Tech/Blueprints/PM_DenseDice.PM_DenseDice")
  (bind _aswbp_score_value (Utilities|Casting|CastToWBP_ScoreValue (UserInterface|GetWidget (Variables|Default|GetWidget))))
  (Default|DisplayValue _aswbp_score_value _value (Utilities|Struct|BreakS_Dice (Variables|Default|GetDiceInfo)))
  (Default|CallEDScoreIncrement (Variables|Default|GetDiceManager) _value))

(event Custom|AfterSettleEffect)

(event Custom|DiceEffect
  (Development|PrintString "Standard")
  (Default|CallEDDieSettled (Variables|Default|GetDiceManager)))

(event EventBeginPlay
  (bind _cube (Variables|Default|GetCube))
  (Class|PhysicsObjectBlueprintLibrary|ApplyRadialImpulse _cube (* (Variables|Default|GetOrigin) (Math|Vector|MakeVector (Math|Random|RandomFloatinRange 0.9 1.1) (Math|Random|RandomFloatinRange 0.9 1.1) (Math|Random|RandomFloatinRange 0.9 1.1))) 5e+02 (* (Math|Random|RandomFloatinRange 2e+02 1e+02) (Physics|GetMass (Variables|Default|GetCube))) "RIF_Constant" false 0.0 false 0.0 1.0)
  (CallFunction|AddTorque _cube)
  (Variables|Default|SetStatic false)
  (bind _returnvalue (Utilities|Time|SetTimerbyEvent (delegate Custom|SetStatic) 0.1 true))
  (Variables|Default|SetTimer _returnvalue))

(event EventTick
  (params (DeltaSeconds :type Float%20%28single-precision%29)))

(fn ConstructionScript)

(fn GetTopFace
  (for _array_element (Transformation|GetAllSocketNames (Variables|Default|GetCube self))
    (if (> (.z (Transformation|GetSocketLocation (Variables|Default|GetCube) _array_element)) (LocalVariables|GetTopFaceHeight))
      (LocalVariables|SetTopFaceHeight (.z (Transformation|GetSocketLocation (Variables|Default|GetCube) _array_element)))
      (LocalVariables|SetTopFaceName _array_element)
      (Transformation|SetWorldRotation (Variables|Default|GetWidget) "0, 0, 0" false false)
      (Transformation|SetWorldLocation (Variables|Default|GetWidget) (+ (Math|Vector|MakeVector (.x (Transformation|GetSocketLocation (Variables|Default|GetCube) _array_element)) (.y (Transformation|GetSocketLocation (Variables|Default|GetCube) _array_element)) (.z (Transformation|GetSocketLocation (Variables|Default|GetCube) _array_element))) "0.000000,0.000000,10.000000") false true)))
  (return (LocalVariables|GetTopFaceName)))

(fn SetRolls
  (Utilities|Time|ClearandInvalidateTimerbyHandle (Variables|Default|GetTimer))
  (bind _name (CallFunction|GetTopFace))
  (return (.Value (Utilities|Map|Find (Variables|Default|GetFaceValues) _name))))

(fn AddTorque
  (params (Cube :type Primitive%20Component%20Object%20Reference))
  (Class|PrimitiveComponent|AddTorqueinDegrees Cube (* (Math|Random|RandomUnitVector) (* (Variables|Default|GetTorque) (Math|Random|RandomFloatinRange 7.5e+03 1.25e+04)) (Physics|GetMass (Variables|Default|GetCube))) "None" false))