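; BP_MirrorDice is a die that mirrors the highest-rolled die once it settles.
; Its AfterSettleEffect reads the highest roll die from DiceManager and copies that die's cube material, world rotation, DiceInfo and the highest roll value.
; It then spawns a RadialBurst effect at its cube's location.
; Roll setup and construction defer to the parent dice class.
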(event EventBeginPlay
  (|CallParentFunction) ; This node is disabled and will not be called.\nDrag off pins to build functionality.
)

(event EventAfterSettleEffect
  (bind _dicemanager (Variables|Default|GetDiceManager))
  (bind _highestrolldice (Variables|/Game/Tech/Blueprints/Dice/BP_DiceManager.BP_DiceManager_C|GetHighestRollDice _dicemanager))
  (bind _cube (Variables|/Game/Tech/Blueprints/Dice/BP_StandardDice.BP_StandardDice_C|GetCube _highestrolldice))
  (Rendering|Material|SetMaterial (Variables|Default|GetCube self) 0 (Rendering|Material|GetMaterial _cube 0))
  (Transformation|SetWorldRotation (Variables|Default|GetCube) (Transformation|GetWorldRotation _cube) false false)
  (Variables|Default|SetDiceInfo (Variables|/Game/Tech/Blueprints/Dice/BP_StandardDice.BP_StandardDice_C|GetDiceInfo (Variables|/Game/Tech/Blueprints/Dice/BP_DiceManager.BP_DiceManager_C|GetHighestRollDice (Variables|Default|GetDiceManager))))
  (Variables|Default|SetValue (Variables|/Game/Tech/Blueprints/Dice/BP_DiceManager.BP_DiceManager_C|GetHighestRollValue (Variables|Default|GetDiceManager)))
  (Niagara|SpawnSystematLocation "/Niagara/DefaultAssets/Templates/Systems/RadialBurst.RadialBurst" (Transformation|GetWorldLocation (Variables|Default|GetCube))))

(fn ConstructionScript
  (|CallParentFunction))

(fn SetRolls
  (|CallParentFunction)
  (return 0))