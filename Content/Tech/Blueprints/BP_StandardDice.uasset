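; Physics die that throws itself on BeginPlay with a randomized radial impulse and torque, then reports the rolled face.
; A looping timer polls the cube's velocity until it is nearly still, then flags it Static and stops.
; GetTopFace picks the highest mesh socket, whose name maps through FaceValues to a number.
; That number becomes the rolled and final value of this die's HeldDice entry in the GameManager, reached through DiceManager.
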(event Custom|SetStatic
  (bind _dicemanager (Variables|Default|GetDiceManager))
  (bind _selfindex (Variables|Default|GetSelfIndex))
  (bind _gamemanager (Variables|/Game/Tech/Blueprints/BP_DiceSpawner.BP_DiceSpawner_C|GetGameManager _dicemanager))
  (bind _helddice (Variables|/Game/Tech/Blueprints/BP_GameManager.BP_GameManager_C|GetHeldDice _gamemanager))
  (bind _output (Utilities|Array|Get(acopy) _helddice _selfindex))
  (bind (_dietype _minvalue _maxvalue _rolledvalue _finalvalue _islocked) (Utilities|Struct|BreakS_Dice _output))
  (if (<= (Math|Vector|VectorLength (Transformation|GetComponentVelocity (Variables|Default|GetCube))) 1e+01)
    (Variables|Default|SetStatic true)
    (Utilities|Time|ClearandInvalidateTimerbyHandle (Variables|Default|GetTimer))
    (bind _name (CallFunction|GetTopFace))
    (|SetBy-RefVar _output (Utilities|Struct|MakeS_Dice _dietype _minvalue _maxvalue (.Value (Utilities|Map|Find (Variables|Default|GetFaceValues) _name)) (.Value (Utilities|Map|Find (Variables|Default|GetFaceValues) _name)) _islocked))))

(event EventBeginPlay
  (bind _cube (Variables|Default|GetCube))
  (Class|PhysicsObjectBlueprintLibrary|ApplyRadialImpulse _cube (* (Variables|Default|GetOrigin) (Math|Vector|MakeVector (Math|Random|RandomFloatinRange 0.9 1.1) (Math|Random|RandomFloatinRange 0.9 1.1) (Math|Random|RandomFloatinRange 0.9 1.1))) 5e+02 (Math|Random|RandomFloatinRange 3.5e+02 6e+02) "RIF_Constant" false 0.0 false 0.0 1.0)
  (Class|PrimitiveComponent|AddTorqueinDegrees _cube (* (Math|Random|RandomUnitVector) (Physics|GetMass (Variables|Default|GetCube)) (* (Variables|Default|GetTorque) 1e+04)) "None" false)
  (Variables|Default|SetStatic false)
  (bind _returnvalue (Utilities|Time|SetTimerbyEvent (delegate Custom|SetStatic) 0.2 true))
  (Variables|Default|SetTimer _returnvalue))

(event EventTick
  (params (DeltaSeconds :type Float%20%28single-precision%29)))

(fn ConstructionScript)

(fn GetTopFace
  (for _array_element (Transformation|GetAllSocketNames (Variables|Default|GetCube self))
    (if (> (.z (Transformation|GetSocketLocation (Variables|Default|GetCube) _array_element)) (LocalVariables|GetTopFaceHeight))
      (LocalVariables|SetTopFaceHeight (.z (Transformation|GetSocketLocation (Variables|Default|GetCube) _array_element)))
      (LocalVariables|SetTopFaceName _array_element)))
  (return (LocalVariables|GetTopFaceName)))