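; Debt display that shows the current debt alongside a running total, both formatted through FormatDebtDisplay.
; Init receives the dice and game managers and hooks the GameManager's debt and total update events.
; Total updates blink the text off for half a second while its value changes.
; A dynamic emissive material tints the total by sampling a color curve at the total-to-debt ratio.
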(event Custom|Init
  (params (DiceManager :type BP%20Dice%20Manager%20Object%20Reference) (GameManager :type BP%20Game%20Manager%20Object%20Reference))
  (Variables|Default|SetDice%20Manager DiceManager)
  (bind _output_get (Variables|Default|SetGame%20Manager GameManager))
  (EventDispatchers|BindEventtoEDDebtUpdated _output_get (delegate Custom|SetDebt))
  (EventDispatchers|AssignEDTotalUpdated _output_get (delegate Custom|ED_TotalUpdated_Event))
  (bind _returnvalue (Rendering|Material|CreateDynamicMaterialInstance "/Game/Art/Emissive/M_EmissiveText_Red.M_EmissiveText_Red" "None" "None" :!class /Script/Engine.KismetMaterialLibrary))
  (bind _output_get_2 (Variables|Default|SetTotalMaterial _returnvalue))
  (Class|Text3DComponent|SetFrontMaterial (Variables|Default|GetCurrentTotal) _output_get_2))

(event Custom|ED_TotalUpdated_Event
  (params (RunningFullTotal :type Integer))
  (bind _output_get (Variables|Default|SetRunning%20Full%20Total RunningFullTotal))
  (Rendering|SetVisibility (Variables|Default|GetCurrentTotal) false false)
  (bind _returnvalue (Class|DebtFormatting|FormatDebtDisplay _output_get))
  (Class|Text3DComponent|SetText (Variables|Default|GetCurrentTotal) (Utilities|Text|FormatText "{1}" _returnvalue))
  (Rendering|Material|SetVectorParameterValue (Variables|Default|GetTotalMaterial) "Color" (Math|Curves|GetLinearColorValue (Variables|Default|GetColor) (/ (Variables|Default|GetRunning%20Full%20Total) (Variables|Default|GetDebt))) :!class /Script/Engine.MaterialInstanceDynamic)
  (Utilities|FlowControl|Delay 0.5)
  (Rendering|SetVisibility (Variables|Default|GetCurrentTotal) true false))

(event Custom|SetDebt
  (params (Debt :type Integer))
  (bind _output_get (Variables|Default|SetDebt Debt))
  (CallFunction|SetCurrentDebt _output_get))

(fn ConstructionScript)

(fn SetCurrentDebt
  (params (DebtAmount :type Integer))
  (bind _returnvalue (Class|DebtFormatting|FormatDebtDisplay DebtAmount))
  (Class|Text3DComponent|SetText (Variables|Default|GetCurrentDebt) (Utilities|Text|FormatText "{1}" _returnvalue)))