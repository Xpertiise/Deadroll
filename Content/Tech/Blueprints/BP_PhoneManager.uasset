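; Manager for the in-game phone that offers random rule modifiers for the dice game.
; On init it caches DT_PhoneRules row names, binds dispatchers and passes itself to the widget; GetRandomRule broadcasts random rows, with repeats possible.
; A selected rule switches on RuleType to modify GameManager or ItemManager values like debt, rolls, dice faces, shop and inventory.
; Ringing swaps the phone's screen material; Answered and Declined are stubs.
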(event Custom|Init
  (bind _outrownames (DataTable|GetDataTableRowNames "/Game/Tech/Data/DT_PhoneRules.DT_PhoneRules"))
  (Variables|Default|SetRow%20Names _outrownames)
  (EventDispatchers|BindEventtoEDRuleSelected (EventDispatchers|CreateEvent :!event Custom|SelectedRule))
  (EventDispatchers|BindEventtoEDPhoneRinging (delegate Custom|CustomEvent))
  (Class|BPIPhoneUI|PassPhoneManager(Message) (Variables|Default|GetWidget) self))

(event Custom|GetRandomRule
  (params (RuleCount :type Integer))
  (bind _row_names (Variables|Default|GetRow%20Names))
  (for _index (range 0 RuleCount)
    (bind _returnvalue (Utilities|GetDataTableRow "/Game/Tech/Data/DT_PhoneRules.DT_PhoneRules" (Utilities|Array|Get(acopy) _row_names (Math|Random|RandomIntegerinRange 0 (- (Utilities|Array|Length _row_names) 1))))
      (:then
        (Utilities|Array|Add (Variables|Default|GetRuleChoices) _returnvalue))))
  (Default|CallEDRulesChosen (Variables|Default|GetRuleChoices))
  (Utilities|Array|Clear (Variables|Default|GetRuleChoices)))

(event Custom|CustomEvent
  (Rule|PhoneRinging))

(event Custom|SelectedRule
  (params (SelectedRule%28s%29 :type S%20Phone%20Call%20Rules%20Structure))
  (switch Utilities|FlowControl|Switch|SwitchonE_RuleType (Utilities|Struct|BreakS_PhoneCallRules SelectedRule%28s%29)
    (:NewEnumerator0
      (Rule|DebtScalingDecrease SelectedRule%28s%29))
    (:NewEnumerator1
      (Rule|DoubleDiceFaces SelectedRule%28s%29))
    (:NewEnumerator2
      (Rule|ExtraRoll SelectedRule%28s%29))
    (:NewEnumerator3
      (Rule|BiggerShop SelectedRule%28s%29))
    (:NewEnumerator4
      (Rule|InventoryIncrease SelectedRule%28s%29))
    (:NewEnumerator6
      (Rule|AutoReroll SelectedRule%28s%29))
    (:NewEnumerator7
      (Rule|ExtraLife SelectedRule%28s%29))))

(fn ConstructionScript)

(fn PhoneRinging
  (Rendering|Material|SetMaterial (Variables|Default|GetPhone) 1 "/Game/Art/M_Screen.M_Screen"))

(fn DebtScalingDecrease
  (params (Rule :type S%20Phone%20Call%20Rules%20Structure))
  (bind _gamemanager (Variables|Default|GetGameManager))
  (Variables|/Game/Tech/Blueprints/BP_GameManager.BP_GameManager_C|SetDebtMultiplier _gamemanager (- (Variables|/Game/Tech/Blueprints/BP_GameManager.BP_GameManager_C|GetDebtMultiplier _gamemanager) (* (.floatvalue Rule) 1.0)))
  (Development|PrintString "Hello"))

(fn BiggerShop
  (params (Rule :type S%20Phone%20Call%20Rules%20Structure))
  (bind _itemmanager (Variables|Default|GetItemManager))
  (Variables|/Game/Tech/Blueprints/BP_ItemManager.BP_ItemManager_C|SetShopItemCount _itemmanager (+ (Variables|/Game/Tech/Blueprints/BP_ItemManager.BP_ItemManager_C|GetShopItemCount _itemmanager) (.floatvalue Rule))))

(fn ExtraRoll
  (params (Rule :type S%20Phone%20Call%20Rules%20Structure))
  (bind _gamemanager (Variables|Default|GetGameManager))
  (Variables|/Game/Tech/Blueprints/BP_GameManager.BP_GameManager_C|SetMaxRolls _gamemanager (+ (.floatvalue Rule) (Variables|/Game/Tech/Blueprints/BP_GameManager.BP_GameManager_C|GetMaxRolls _gamemanager))))

(fn AutoReroll
  (params (Rule :type S%20Phone%20Call%20Rules%20Structure))
  (Variables|/Game/Tech/Blueprints/BP_GameManager.BP_GameManager_C|SetAutoReroll%20Enabled (Variables|Default|GetGameManager) true))

(fn ExtraLife
  (params (Rule :type S%20Phone%20Call%20Rules%20Structure))
  (Variables|/Game/Tech/Blueprints/BP_GameManager.BP_GameManager_C|SetExtraLife (Variables|Default|GetGameManager) true))

(fn DoubleDiceFaces
  (params (Rule :type S%20Phone%20Call%20Rules%20Structure))
  (bind _gamemanager (Variables|Default|GetGameManager))
  (Variables|/Game/Tech/Blueprints/BP_GameManager.BP_GameManager_C|SetFaceMulti _gamemanager (* (Variables|/Game/Tech/Blueprints/BP_GameManager.BP_GameManager_C|GetFaceMulti _gamemanager) (.floatvalue Rule))))

(fn InventoryIncrease
  (params (Rule :type S%20Phone%20Call%20Rules%20Structure))
  (bind _gamemanager (Variables|Default|GetGameManager))
  (bind _gamedata (Variables|/Game/Tech/Blueprints/BP_GameManager.BP_GameManager_C|GetGameData _gamemanager))
  (Utilities|Struct|SetmembersinS_UIStruct _gamedata (Math|Float|Truncate (+ (.floatvalue Rule) (Utilities|Struct|BreakS_UIStruct _gamedata)))))

(fn Answered
  (Development|PrintString "Phone Answered"))

(fn Declined)